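; BP_Block_Magma is a destructible magma block that hurts the first-person player character on contact.
; Entering its box trigger deals an initial hit, then a looping timer applies small repeated damage until the player leaves.
; StartDestroy plays a rate-scaled timeline driving a dynamic material's DestroyAmount, then removes the block through GI_BlockGame and destroys the actor.
; StopDestroy cancels this and resets the material.
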(event `self.ReceiveBeginPlay`
  (bind _block (`self.Block`))
  (bind _returnvalue (`PrimitiveComponent.CreateDynamicMaterialInstance` _block 0 (`PrimitiveComponent.GetMaterial` _block 0) "None"))
  (set `self.Block Mat` _returnvalue)
  (`TimelineComponent.SetPlayRate` (`self.DestroyTimeline`) (`self.DestroyRate`)))

(event `StartDestroy`
  ;[1 1 1] Destroy Blocks
  (bind (_direction _destroyamount) (`Timeline|DestroyTimeline` :!via `PlayFromStart` :!label _label)
    (:`Update`
      (`MaterialInstanceDynamic.SetScalarParameterValue` (`self.Block Mat`) "DestroyAmount" _destroyamount))
    (:`Finished`
      (`/Game/FirstPerson/Blueprints/GI_BlockGame.RemoveBlock` (cast `/Game/FirstPerson/Blueprints/GI_BlockGame` (`GameplayStatics.GetGameInstance`) :!pure true) (`SceneComponent.K2_GetComponentLocation` (`self.DefaultSceneRoot`)))
      (`self.K2_DestroyActor`))))

(event `StopDestroy`
  ;[1 1 1] Destroy Blocks
  (`MaterialInstanceDynamic.SetScalarParameterValue` (`self.Block Mat`) "DestroyAmount" 0.0)
  (goto _label :!via `Stop`))

(event `self.Box.OnComponentBeginOverlap`
  (params (OverlappedComponent :type "PrimitiveComponent Object Reference") (OtherActor :type "Actor Object Reference") (OtherComp :type "PrimitiveComponent Object Reference") (OtherBodyIndex :type Integer) (bFromSweep :type Boolean) (SweepResult :type "HitResult Structure (by ref)"))
  (bind _asbp_first_person_character (cast `/Game/FirstPerson/Blueprints/BP_FirstPersonCharacter` OtherActor))
  (bind _output_get (set `self.PlayerRef` _asbp_first_person_character))
  (`/Game/FirstPerson/Blueprints/BP_FirstPersonCharacter.Damage` _output_get 11)
  (bind _returnvalue (`KismetSystemLibrary.K2_SetTimerDelegate` (delegate `LoopDamage`) 0.1 true))
  (set `self.Timer Handle` _returnvalue))

(event `LoopDamage`
  (`/Game/FirstPerson/Blueprints/BP_FirstPersonCharacter.Damage` (`self.PlayerRef`) 1))

(event `self.Box.OnComponentEndOverlap`
  (params (OverlappedComponent :type "PrimitiveComponent Object Reference") (OtherActor :type "Actor Object Reference") (OtherComp :type "PrimitiveComponent Object Reference") (OtherBodyIndex :type Integer))
  (cast `/Game/FirstPerson/Blueprints/BP_FirstPersonCharacter` OtherActor)
  (`KismetSystemLibrary.K2_ClearAndInvalidateTimerHandle` (`self.Timer Handle`)))

(fn `UserConstructionScript`)