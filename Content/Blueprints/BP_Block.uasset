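; BP_Block is a destructible block that is mined over time and added to the player's inventory.
; On BeginPlay it creates a dynamic material instance and applies its destroy rate to a timeline, which drives the DestroyAmount parameter during StartDestroy.
; When the timeline finishes, it removes its location from GI_BlockGame, gives its class to the first-person character and destroys itself.
; StopDestroy halts the timeline and resets the visual.
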(event `self.ReceiveBeginPlay`
  (bind _block (`self.Block`))
  (bind _returnvalue (`PrimitiveComponent.CreateDynamicMaterialInstance` _block 0 (`PrimitiveComponent.GetMaterial` _block 0) "None"))
  (set `self.Block Mat` _returnvalue)
  (`TimelineComponent.SetPlayRate` (`self.DestroyTimeline`) (`self.DestroyRate`)))

(event `StartDestroy`
  ;[1 1 1] Destroy Blocks
  (bind (_direction _destroyamount) (`Timeline|DestroyTimeline` :!via `PlayFromStart` :!label _label)
    (:`Update`
      (`MaterialInstanceDynamic.SetScalarParameterValue` (`self.Block Mat`) "DestroyAmount" _destroyamount))
    (:`Finished`
      (`/Game/FirstPerson/Blueprints/GI_BlockGame.RemoveBlock` (cast `/Game/FirstPerson/Blueprints/GI_BlockGame` (`GameplayStatics.GetGameInstance`) :!pure true) (`SceneComponent.K2_GetComponentLocation` (`self.DefaultSceneRoot`)))
      (bind _asbp_first_person_character (cast `/Game/FirstPerson/Blueprints/BP_FirstPersonCharacter` (`GameplayStatics.GetPlayerCharacter` 0))
        (:`then`
          (`/Game/FirstPerson/Blueprints/BP_FirstPersonCharacter.AddBlockToInventory` _asbp_first_person_character (`GameplayStatics.GetObjectClass` self)))
        (:`CastFailed`
          _))
      (`self.K2_DestroyActor`))))

(event `StopDestroy`
  ;[1 1 1] Destroy Blocks
  (`MaterialInstanceDynamic.SetScalarParameterValue` (`self.Block Mat`) "DestroyAmount" 0.0)
  (goto _label :!via `Stop`))

(fn `UserConstructionScript`)